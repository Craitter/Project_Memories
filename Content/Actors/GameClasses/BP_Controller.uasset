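; Player controller that switches input and participant state around Mountea dialogue sessions.
; When a dialogue initializes, it sets the pawn's dialogue participant to Active and switches to mouse-locked UI-only input with a widget from the dialogue context as focus target.
; On close, it restores game-only input, re-enables the participant and resets the MemoriesCharacter's interaction trace.
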(event OnDialogueStarted(MounteaDialogueManager)
  (params (Context :type Mountea%20Dialogue%20Context%20Object%20Reference)))

(event OnDialogueClosed(MounteaDialogueManager)
  (params (Context :type Mountea%20Dialogue%20Context%20Object%20Reference))
  (Input|SetInputModeGameOnly self false)
  (Class|MounteaDialogueParticipant|SetParticipantState (Actor|GetComponentbyClass (Pawn|GetControlledPawn) "/Script/MounteaDialogueSystem.MounteaDialogueParticipant") "EDPS_Enabled")
  (bind _asmemories_character (Utilities|Casting|CastToMemoriesCharacter (Pawn|GetControlledPawn self)))
  (Class|MemoriesCharacter|ResetInteractionTrace _asmemories_character))

(event OnDialogueInitialized(MounteaDialogueManager)
  (params (Context :type Mountea%20Dialogue%20Context%20Object%20Reference))
  (Class|MounteaDialogueParticipant|SetParticipantState (Actor|GetComponentbyClass (Pawn|GetControlledPawn) "/Script/MounteaDialogueSystem.MounteaDialogueParticipant") "EDPS_Active")
  (bind _returnvalue (Class|MounteaDialogueManagerInterface|GetDialogueWidget(Message) Context))
  (Input|SetInputModeUIOnly self _returnvalue "LockAlways" true))

(event OnDialogueNodeStarted(MounteaDialogueManager)
  (params (Context :type Mountea%20Dialogue%20Context%20Object%20Reference)))

(event EventBeginPlay)

(event EventTick
  (params (DeltaSeconds :type Float%20%28single-precision%29)))

(fn ConstructionScript)